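; BP_ColorPuzzle is a possessable color puzzle that unlocks once its colors, canvas and brush have all been collected.
; It binds to the OnCollected event of each of the three references, sets a matching flag, then recomputes CanBePossessed as the AND of all three.
; The exit-puzzle input action calls ReturnToCharacter, and the puzzle gameplay itself is not in this graph.
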(event `self.ReceiveBeginPlay`
  (add `/Game/Blueprints/Tmp/BP_ColorPuzzleRequisite.OnCollected` (`self.Colors`) (delegate `OnCollected_Event`))
  (add `/Game/Blueprints/Tmp/BP_ColorPuzzleRequisite.OnCollected` (`self.Canvas`) (delegate `OnCollected_Event_0`))
  (add `/Game/Blueprints/Tmp/BP_ColorPuzzleRequisite.OnCollected` (`self.Brush`) (delegate `OnCollected_Event_1`)))

(event `OnCollected_Event`
  (set `self.HasColors` true)
  (`self.UpdateCanBePossessed`))

(event `OnCollected_Event_0`
  (set `self.HasCanvas` true)
  (`self.UpdateCanBePossessed`))

(event `OnCollected_Event_1`
  (set `self.HasBrush` true)
  (`self.UpdateCanBePossessed`))

(event `EnhancedInput|/Game/Input/Actions/IA_ExitPuzzle`
  (params (ActionValue :type Boolean) (ElapsedSeconds :type "Float (double-precision)") (TriggeredSeconds :type "Float (double-precision)") (InputAction :type "InputAction Object Reference" :default "/Game/Input/Actions/IA_ExitPuzzle.IA_ExitPuzzle"))
  (:`Triggered`
    (`self.Return to Character`)))

(fn `UpdateCanBePossessed`
  (set `self.CanBePossessed` (and (`self.HasColors`) (`self.HasCanvas`) (`self.HasBrush`))))

(fn `UserConstructionScript`
  (`parent.UserConstructionScript`))