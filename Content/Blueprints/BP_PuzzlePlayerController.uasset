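; Player controller for a first-person puzzle game that routes Enhanced Input to the possessed BP_FirstPersonCharacter.
; BeginPlay adds the IMC_FirstPerson mapping context, and possession caches the cast character reference.
; Input actions drive that character's look, jump and TryINteract call, plus movement rotated into world space by its actor transform.
; An alternative forward/right-vector movement calculation is left disconnected.
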(event `self.ReceiveBeginPlay`
  (`EnhancedInputSubsystemInterface.AddMappingContext` (subsystem `EnhancedInputLocalPlayerSubsystem`) "/Game/Input/IMC_FirstPerson.IMC_FirstPerson" 0 (struct)))

(event `self.ReceivePossess`
  (params (PossessedPawn :type "Pawn Object Reference"))
  (bind _asbp_first_person_character (cast `/Game/Blueprints/BP_FirstPersonCharacter` PossessedPawn))
  (set `self.Possessed Character` _asbp_first_person_character))

(event `EnhancedInput|/Game/Input/Actions/IA_Look`
  (params (ActionValue :type "Vector2D Structure") (ElapsedSeconds :type "Float (double-precision)") (TriggeredSeconds :type "Float (double-precision)") (InputAction :type "InputAction Object Reference" :default "/Game/Input/Actions/IA_Look.IA_Look"))
  (:`Triggered`
    (`Pawn.AddControllerYawInput` (`self.Possessed Character`) ActionValue_X)
    (`Pawn.AddControllerPitchInput` (`self.Possessed Character`) ActionValue_Y)))

(event `EnhancedInput|/Game/Input/Actions/IA_Move`
  (params (ActionValue :type "Vector2D Structure") (ElapsedSeconds :type "Float (double-precision)") (TriggeredSeconds :type "Float (double-precision)") (InputAction :type "InputAction Object Reference" :default "/Game/Input/Actions/IA_Move.IA_Move"))
  (:`Triggered`
    (`Pawn.AddMovementInput` (`self.Possessed Character`) (`KismetMathLibrary.TransformDirection` (`self.GetTransform` (`self.Possessed Character`)) (`KismetMathLibrary.MakeVector` ActionValue_X ActionValue_Y)) 1.0 false)))

(event `EnhancedInput|/Game/Input/Actions/IA_Jump`
  (params (ActionValue :type Boolean) (ElapsedSeconds :type "Float (double-precision)") (TriggeredSeconds :type "Float (double-precision)") (InputAction :type "InputAction Object Reference" :default "/Game/Input/Actions/IA_Jump.IA_Jump"))
  (:`Triggered`
    (`Character.Jump` (`self.Possessed Character`))))

(event `EnhancedInput|/Game/Input/Actions/IA_Interact`
  (params (ActionValue :type Boolean) (ElapsedSeconds :type "Float (double-precision)") (TriggeredSeconds :type "Float (double-precision)") (InputAction :type "InputAction Object Reference" :default "/Game/Input/Actions/IA_Interact.IA_Interact"))
  (:`Triggered`
    (`/Game/Blueprints/BP_FirstPersonCharacter.TryINteract` (`self.Possessed Character`))))

(fn `UserConstructionScript`)