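; BP_PickupTarget is an interactable receiver that accepts a pickup of one desired class.
; Interact checks the offered pickup's exact class, attaches a match at TargetTransform, sets HasReceivedPickup and returns true.
; Once filled, each further interaction calls Rotate, which turns the root component by a fixed 45-degree step.
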(fn `Interact`
  (params (PlayerCharacter :type "/Game/Blueprints/BP_FirstPersonCharacter Object Reference") (Pickup :type "/Game/Blueprints/Pickups/BP_PickupActor Object Reference"))
  (returns (UsedUpPickup :type Boolean))
  (if (`self.HasReceivedPickup`)
    (`self.Rotate`)
    (else
      (`/Engine/EditorBlueprintResources/StandardMacros.IsValid` Pickup
        (:`Is Valid`
          (if (== (`GameplayStatics.GetObjectClass` Pickup) (`self.DesiredPickup`))
            (`/Game/Blueprints/Pickups/BP_PickupActor.AttachTo` Pickup (`self.TargetTransform`))
            (set `self.HasReceivedPickup` true)
            (return true)))))))

(fn `Rotate`
  (`SceneComponent.K2_AddRelativeRotation` (`self.DefaultSceneRoot`) (struct :`Yaw` 45.0) false false))

(fn `UserConstructionScript`)