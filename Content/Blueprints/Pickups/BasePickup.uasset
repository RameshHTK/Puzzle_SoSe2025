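; Base pickup actor that can be picked up, dropped or placed at a target transform.
; Pickup disables mesh physics and collision, then snaps the actor to the given scene component while keeping world scale.
; Dropping detaches it in world space and restores both through a shared toggle function.
; Placing detaches it, keeps both disabled, and moves it to the target location and rotation.
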(event `/Game/Blueprints/Pickups/BPI_Pickup.GetPickedUp`
  (params (SceneComponent :type "SceneComponent Object Reference"))
  (`self.SetPhysiscsAndCollision` false)
  (`self.K2_AttachToComponent` SceneComponent "None" "SnapToTarget" "SnapToTarget" "KeepWorld"))

(event `/Game/Blueprints/Pickups/BPI_Pickup.GetDropped`
  (`self.DetachFromPlayer`)
  (`self.SetPhysiscsAndCollision` true))

(event `/Game/Blueprints/Pickups/BPI_Pickup.GetPlaced`
  (params (TargetTransform :type "Transform Structure"))
  (`self.K2_DetachFromActor` "KeepWorld" "KeepWorld" "KeepWorld")
  (`self.SetPhysiscsAndCollision` false)
  (`self.K2_SetActorLocationAndRotation` TargetTransform_Location TargetTransform_Rotation))

(fn `DetachFromPlayer`
  (`self.K2_DetachFromActor` "KeepWorld" "KeepWorld" "KeepWorld"))

(fn `SetPhysiscsAndCollision`
  (params (Enabled :type Boolean))
  (if Enabled
    (`PrimitiveComponent.SetCollisionEnabled` (`self.StaticMesh`) "QueryAndPhysics")
    (`PrimitiveComponent.SetSimulatePhysics` (`self.StaticMesh`) true)
    (else
      (`PrimitiveComponent.SetSimulatePhysics` (`self.StaticMesh`) false)
      (`PrimitiveComponent.SetCollisionEnabled` (`self.StaticMesh`) "NoCollision"))))

(fn `UserConstructionScript`)