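; BP_PickupActor is a pickup actor whose static mesh can be attached to a given component and later dropped.
; AttachTo turns off the mesh's physics and collision, then attaches to the component, snapping location and rotation while keeping world scale.
; Drop detaches with world transform intact, then restores collision and physics simulation.
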(event `AttachTo`
  (params (ComponentToAttachTo :type "SceneComponent Object Reference"))
  (`PrimitiveComponent.SetSimulatePhysics` (`self.StaticMesh`) false)
  (`PrimitiveComponent.SetCollisionEnabled` (`self.StaticMesh`) "NoCollision")
  (`self.K2_AttachToComponent` ComponentToAttachTo "None" "SnapToTarget" "SnapToTarget" "KeepWorld"))

(event `Drop`
  (`self.K2_DetachFromActor` "KeepWorld" "KeepWorld" "KeepWorld")
  (`PrimitiveComponent.SetCollisionEnabled` (`self.StaticMesh`) "QueryAndPhysics")
  (`PrimitiveComponent.SetSimulatePhysics` (`self.StaticMesh`) true))

(fn `UserConstructionScript`)