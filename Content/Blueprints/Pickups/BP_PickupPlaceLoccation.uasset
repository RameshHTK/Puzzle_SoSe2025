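; BP_PickupPlaceLoccation is a placement spot that accepts one pickup of a configured class.
; On BeginPlay, its text render shows the display name of AcceptedPickupClass.
; Interact requires an empty slot and an exact class match, then stores the pickup as PlacedPickup, passes it the PickupPivot world transform through GetPlacedMessage, and returns true.
; Nothing in these graphs clears the slot.
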(event `self.ReceiveBeginPlay`
  (`TextRenderComponent.K2_SetText` (`self.TextRender`) (`KismetTextLibrary.Conv_StringToText` (`KismetSystemLibrary.GetClassDisplayName` (`self.AcceptedPickupClass`)))))

(fn `Interact`
  (params (PlayerCharacter :type "/Game/Blueprints/BP_FirstPersonCharacter Object Reference") (Pickup :type "Actor Object Reference"))
  (returns (UsedPickup :type Boolean))
  (`/Engine/EditorBlueprintResources/StandardMacros.IsValid` (`self.PlacedPickup`)
    (:`Is Not Valid`
      (if (== (`GameplayStatics.GetObjectClass` Pickup) (`self.AcceptedPickupClass`))
        (bind _output_get (set `self.PlacedPickup` Pickup))
        (`/Engine/EditorBlueprintResources/StandardMacros.IsValid` _output_get
          (:`Is Valid`
            (message `/Game/Blueprints/Pickups/BPI_Pickup.GetPlaced` (`self.PlacedPickup`) (`SceneComponent.K2_GetComponentToWorld` (`self.PickupPivot`)))
            (return true))
          (:`Is Not Valid`
            (return false)))))))

(fn `UserConstructionScript`)