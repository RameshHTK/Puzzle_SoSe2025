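; BP_LaserPossessable is a possessable laser puzzle piece that can emit, receive or redirect a beam, with look input rotating its yaw.
; Sources trace forward every tick, sizing the Niagara beam to the hit and notifying any laser piece struck.
; Box hits fire a callback and chain through redirectors, with a game-time stamp preventing repeat hits within a frame.
; Unlit non-sources switch their beam off, and exit input returns to the character.
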(event `self.ReceiveBeginPlay`
  ;[1 1 1] Enable visuals of source Laser
  (`self.SetVFX Enabled` (`self.IsLaserSource`)))

(event `self.ReceiveTick`
  (params (DeltaSeconds :type "Float (single-precision)"))
  ;[1 1 1] If source: Emit laser on tick
  (if (`self.IsLaserSource`)
    (`self.EmitLaser`)
    (else
      ;[1 1 1] Disable Laser if hasn't been hit recently
      (if (`self.TimeHasPassedSinceLastHit`)
        (`self.SetVFX Enabled` false)))))

(event `GetHitByLaser`
  (params (HitComponent :type "PrimitiveComponent Object Reference"))
  ;[1 1 1] Receive Laser
  (if (== HitComponent (`self.Box`))
    (if (`self.TimeHasPassedSinceLastHit`)
      (set `self.LastHitTime` (`KismetSystemLibrary.GetGameTimeInSeconds`))
      (`self.OnHitByLaser`)
      (if (`self.CanRedirectLight`)
        (`self.SetVFX Enabled` true)
        (`self.EmitLaser`)))))

(event `EnhancedInput|/Game/Input/Actions/IA_Look`
  (params (ActionValue :type "Vector2D Structure") (ElapsedSeconds :type "Float (double-precision)") (TriggeredSeconds :type "Float (double-precision)") (InputAction :type "InputAction Object Reference" :default "/Game/Input/Actions/IA_Look.IA_Look"))
  ;[0.1024 0.7107 1] Controls
  (:`Triggered`
    (`self.K2_AddActorLocalRotation` (`KismetMathLibrary.MakeRotator` 0.0 0.0 (* ActionValue_X (`GameplayStatics.GetWorldDeltaSeconds`) (`self.RotationSpeed`))))))

(event `EnhancedInput|/Game/Input/Actions/IA_ExitPuzzle`
  (params (ActionValue :type Boolean) (ElapsedSeconds :type "Float (double-precision)") (TriggeredSeconds :type "Float (double-precision)") (InputAction :type "InputAction Object Reference" :default "/Game/Input/Actions/IA_ExitPuzzle.IA_ExitPuzzle"))
  ;[0.1024 0.7107 1] Controls
  ;;[1 1 1] Exit Puzle
  (:`Triggered`
    (`self.Return to Character`)))

(fn `CheckForLaserHit`
  (returns (HitSomething :type Boolean) (DistanceToHit :type "Float (double-precision)") (`HitLaser Possessable` :type "/Game/Blueprints/Laser/BP_LaserPossessable Object Reference") (HitComponent :type "PrimitiveComponent Object Reference"))
  (bind _laserorigin (`self.LaserOrigin`))
  (bind _returnvalue (`SceneComponent.K2_GetComponentLocation` _laserorigin))
  (bind (_outhit _returnvalue_2) (`KismetSystemLibrary.LineTraceSingleForObjects` _returnvalue (+ _returnvalue (* (`SceneComponent.GetForwardVector` _laserorigin) (`self.LaserRange`))) (`|MakeArray` "ObjectTypeQuery1" "ObjectTypeQuery2" "ObjectTypeQuery3" "ObjectTypeQuery4" :!type "EObjectTypeQuery Enum")))
  (if _returnvalue_2
    (bind (_bblockinghit _binitialoverlap _time _distance _location _impactpoint _normal _impactnormal _physmat _hitactor _hitcomponent) (`GameplayStatics.BreakHitResult` _outhit))
    (bind _asbp_laser_possessable (cast `/Game/Blueprints/Laser/BP_LaserPossessable` _hitactor)
      (:`then`
        _)
      (:`CastFailed`
        _))
    (return true (`KismetMathLibrary.VSize` (- _impactpoint (`SceneComponent.K2_GetComponentLocation` (`self.LaserOrigin`)))) _asbp_laser_possessable _hitcomponent)
    (else
      (return false 0.0 null null))))

(fn `EmitLaser`
  (bind (_hitsomething _distancetohit _hitlaser_possessable _hitcomponent) (`self.CheckForLaserHit`))
  (if _hitsomething
    (`NiagaraComponent.SetVariableFloat` (`self.NS_Laser2`) "LaserLength" _distancetohit)
    (`/Engine/EditorBlueprintResources/StandardMacros.IsValid` _hitlaser_possessable
      (:`Is Valid`
        (`self.GetHitByLaser` _hitlaser_possessable _hitcomponent)))))

(fn `SetVFX Enabled`
  (params (IsEnabled :type Boolean))
  (bind _ns_laser2 (`self.NS_Laser2`))
  (if IsEnabled
    (`ActorComponent.Activate` _ns_laser2 false)
    (else
      (`ActorComponent.Deactivate` _ns_laser2))))

(fn `TimeHasPassedSinceLastHit`
  (returns (ReturnValue :type Boolean))
  (return (> (`KismetSystemLibrary.GetGameTimeInSeconds`) (`self.LastHitTime`))))

(fn `UserConstructionScript`
  (`parent.UserConstructionScript`)
  (`self.SetVFX Enabled` (`self.IsLaserSource`)))