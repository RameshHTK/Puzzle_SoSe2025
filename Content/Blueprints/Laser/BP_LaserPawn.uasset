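; BP_LaserPawn is a pawn that fits the length of a Niagara laser beam to whatever it hits.
; Each tick it runs an object-type line trace forward from LaserOrigin, covering world, pawn and physics-body objects.
; On a hit, it writes the distance to the impact point into the LaserLength variable of NSLaser.
; A miss leaves LaserLength unchanged, so the beam keeps its last set length.
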(event `self.ReceiveBeginPlay`)

(event `self.ReceiveTick`
  (params (DeltaSeconds :type "Float (single-precision)"))
  (bind _laserorigin (`self.LaserOrigin`))
  (bind _returnvalue (`SceneComponent.K2_GetComponentLocation` _laserorigin))
  (bind (_outhit _returnvalue_2) (`KismetSystemLibrary.LineTraceSingleForObjects` _returnvalue (+ _returnvalue (* (`SceneComponent.GetForwardVector` _laserorigin) 5000.0)) (`|MakeArray` "ObjectTypeQuery1" "ObjectTypeQuery2" "ObjectTypeQuery3" "ObjectTypeQuery4" :!type "EObjectTypeQuery Enum")))
  (if _returnvalue_2
    (`NiagaraComponent.SetVariableFloat` (`self.NS_Laser`) "LaserLength" (`KismetMathLibrary.VSize` (- (`.ImpactPoint` (`GameplayStatics.BreakHitResult` _outhit)) (`SceneComponent.K2_GetComponentLocation` (`self.LaserOrigin`)))))))

(fn `UserConstructionScript`)