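; Base interactable pawn that the player can possess on interaction and later leave to return to their character.
; Both transitions blend the view target, delay for the blend, then switch possession and swap Enhanced Input mapping contexts.
; On exit, it moves the character to ground traced below the child's expected camera component, matching the camera's rotation.
; A helper toggles a highlight overlay material on a given mesh.
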(event `/Game/Blueprints/InteractionInterface.Interact`
  (params (PlayerCharacter :type "/Game/Blueprints/BP_FirstPersonCharacter Object Reference"))
  ;[1 1 1] Get interacted with
  (set `self.Player Character` PlayerCharacter)
  (`self.GetPossessed`))

(event `GetPossessed`
  ;[1 1 1] Get Possessed
  (`EnhancedInputSubsystemInterface.RemoveMappingContext` (pcsubsystem `EnhancedInputLocalPlayerSubsystem` (`GameplayStatics.GetPlayerController` 0)) (`self.CharacterMappingContext`) (struct))
  (`PlayerController.SetViewTargetWithBlend` (`GameplayStatics.GetPlayerController` 0) self (`self.SmoothPossessDuration`) "VTBlend_Linear" 0.0 false)
  (`KismetSystemLibrary.Delay` (`self.SmoothPossessDuration`))
  (`Controller.Possess` (`GameplayStatics.GetPlayerController` 0) self)
  (`EnhancedInputSubsystemInterface.AddMappingContext` (pcsubsystem `EnhancedInputLocalPlayerSubsystem` (`GameplayStatics.GetPlayerController` 0)) (`self.Mapping Context`) 0 (struct)))

(event `Return to Character`
  ;[1 1 1] Possess Character
  (`self.PositionPlayerCharacter`)
  (`EnhancedInputSubsystemInterface.RemoveMappingContext` (pcsubsystem `EnhancedInputLocalPlayerSubsystem` (`GameplayStatics.GetPlayerController` 0)) (`self.Mapping Context`) (struct))
  (`PlayerController.SetViewTargetWithBlend` (`GameplayStatics.GetPlayerController` 0) (`self.Player Character`) (`self.SmoothPossessDuration`) "VTBlend_Linear" 0.0 false)
  (`KismetSystemLibrary.Delay` (`self.SmoothPossessDuration`))
  (`EnhancedInputSubsystemInterface.AddMappingContext` (pcsubsystem `EnhancedInputLocalPlayerSubsystem` (`GameplayStatics.GetPlayerController` 0)) (`self.CharacterMappingContext`) 0 (struct))
  (`Controller.Possess` (`GameplayStatics.GetPlayerController` 0) (`self.Player Character`)))

(fn `PositionPlayerCharacter`
  (locals (Cam :type "CameraComponent Object Reference"))
  (bind _returnvalue (`SceneComponent.K2_GetComponentLocation` (`local.Cam`)))
  (bind _output_get (set `local.Cam` (`self.GetComponentByClass` "/Script/Engine.CameraComponent")))
  (`/Engine/EditorBlueprintResources/StandardMacros.IsValid` _output_get
    (:`Is Valid`
      (`self.K2_SetActorRotation` (`self.Player Character`) (`SceneComponent.K2_GetComponentRotation` (`local.Cam`)) false)
      (bind (_outhit _returnvalue_2) (`KismetSystemLibrary.LineTraceSingleForObjects` :`Start` _returnvalue :`End` (- _returnvalue (0.0 0.0 300.0)) :`ObjectTypes` (`|MakeArray` "ObjectTypeQuery1" "ObjectTypeQuery2" :!type "EObjectTypeQuery Enum") :`DrawTime` 10.0))
      (if _returnvalue_2
        (`self.K2_SetActorLocation` (`self.Player Character`) (+ (`.Location` (`GameplayStatics.BreakHitResult` _outhit)) (`KismetMathLibrary.MakeVector` 0.0 0.0 (+ (`CapsuleComponent.CapsuleHalfHeight` (`Character.CapsuleComponent` (`self.Player Character`))) 1.0))) false false)))
    (:`Is Not Valid`
      (`KismetSystemLibrary.PrintString` "BP_InteractablePossessable assumes child has camera component but found none!" true true (struct :`R` 1.0 :`G` 0.042674 :`A` 1.0) 8.0))))

(fn `SetHighlight`
  (params (bEnabled :type Boolean) (MeshComp :type "MeshComponent Object Reference"))
  (`MeshComponent.SetOverlayMaterial` MeshComp (select `bool` bEnabled :`true` "/Game/Materials/MI_ButtonHighlight.MI_ButtonHighlight" :!type "MaterialInterface Object Reference")))

(fn `UserConstructionScript`)