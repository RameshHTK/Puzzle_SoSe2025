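; BP_RotationLock is an interactable combination lock puzzle built from four rotating symbol discs.
; Input actions move a clamped, highlighted selection left or right and rotate the selected disc up or down.
; On interact, it compares each disc's current symbol to CorrectCombination, printing the result and returning to the character when correct.
; The parent class supplies the base interact and return-to-character behavior, extended here to toggle the highlight.
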(event `self.ReceiveBeginPlay`
  ;[1 1 1] Setup
  (`parent.ReceiveBeginPlay`)
  (set `self.Discs` (`|MakeArray` (`self.BP_RotationLock_Disc`) (`self.BP_RotationLock_Disc1`) (`self.BP_RotationLock_Disc2`) (`self.BP_RotationLock_Disc3`))))

(event `/Game/Blueprints/InteractionInterface.Interact`
  (params (PlayerCharacter :type "/Game/Blueprints/BP_FirstPersonCharacter Object Reference"))
  (`parent.Interact` PlayerCharacter)
  (`self.SetSelectedDiscHighlight` true))

(event `EnhancedInput|/Game/Input/Actions/IA_ExitPuzzle`
  (params (ActionValue :type Boolean) (ElapsedSeconds :type "Float (double-precision)") (TriggeredSeconds :type "Float (double-precision)") (InputAction :type "InputAction Object Reference" :default "/Game/Input/Actions/IA_ExitPuzzle.IA_ExitPuzzle"))
  (:`Triggered`
    (`self.Return to Character`)))

(event `self.Return to Character`
  (`parent.Return to Character`)
  (`self.SetSelectedDiscHighlight` false))

(event `EnhancedInput|/Game/Input/Actions/IA_NavigateLeft`
  (params (ActionValue :type Boolean) (ElapsedSeconds :type "Float (double-precision)") (TriggeredSeconds :type "Float (double-precision)") (InputAction :type "InputAction Object Reference" :default "/Game/Input/Actions/IA_NavigateLeft.IA_NavigateLeft"))
  (:`Triggered`
    (`self.ChangeSelectedDisc` false)))

(event `EnhancedInput|/Game/Input/Actions/IA_NavigateRight`
  (params (ActionValue :type Boolean) (ElapsedSeconds :type "Float (double-precision)") (TriggeredSeconds :type "Float (double-precision)") (InputAction :type "InputAction Object Reference" :default "/Game/Input/Actions/IA_NavigateRight.IA_NavigateRight"))
  (:`Triggered`
    (`self.ChangeSelectedDisc` true)))

(event `EnhancedInput|/Game/Input/Actions/IA_NavigateUp`
  (params (ActionValue :type Boolean) (ElapsedSeconds :type "Float (double-precision)") (TriggeredSeconds :type "Float (double-precision)") (InputAction :type "InputAction Object Reference" :default "/Game/Input/Actions/IA_NavigateUp.IA_NavigateUp"))
  (:`Triggered`
    (`/Game/Blueprints/RotationLock/BP_RotationLock_Disc.Rotate` (`self.GetSelectedDisc`) true)))

(event `EnhancedInput|/Game/Input/Actions/IA_NavigateDown`
  (params (ActionValue :type Boolean) (ElapsedSeconds :type "Float (double-precision)") (TriggeredSeconds :type "Float (double-precision)") (InputAction :type "InputAction Object Reference" :default "/Game/Input/Actions/IA_NavigateDown.IA_NavigateDown"))
  (:`Triggered`
    (`/Game/Blueprints/RotationLock/BP_RotationLock_Disc.Rotate` (`self.GetSelectedDisc`) false)))

(event `EnhancedInput|/Game/Input/Actions/IA_Interact`
  (params (ActionValue :type Boolean) (ElapsedSeconds :type "Float (double-precision)") (TriggeredSeconds :type "Float (double-precision)") (InputAction :type "InputAction Object Reference" :default "/Game/Input/Actions/IA_Interact.IA_Interact"))
  (:`Triggered`
    (if (`self.EvaluateCombination`)
      (`KismetSystemLibrary.PrintString` "Correct!" true true (struct :`G` 1.0 :`B` 0.196204 :`A` 1.0))
      (`self.Return to Character`)
      (else
        (`KismetSystemLibrary.PrintString` "Wrong!" true true (struct :`R` 1.0 :`B` 0.008382 :`A` 1.0))))))

(fn `ChangeSelectedDisc`
  (params (bRight :type Boolean))
  (`self.SetSelectedDiscHighlight` false)
  (set `self.SelectedDiscIndex` (`KismetMathLibrary.Clamp` (+ (`self.SelectedDiscIndex`) (`KismetMathLibrary.SelectInt` 1 -1 bRight)) 0 (`KismetArrayLibrary.Array_LastIndex` (`self.Discs`))))
  (`self.SetSelectedDiscHighlight` true))

(fn `EvaluateCombination`
  (returns (CombinationCorrect :type Boolean))
  (for (_array_element _array_index) (`self.Discs`)
    (if (`|EnumInequality` (`/Game/Blueprints/RotationLock/BP_RotationLock_Disc.GetCurrentSymbol` _array_element) (`|GetArrayItem` (`self.CorrectCombination`) _array_index))
      (return false)))
  (return true))

(fn `GetSelectedDisc`
  (returns (Output :type "/Game/Blueprints/RotationLock/BP_RotationLock_Disc Object Reference"))
  (return (`|GetArrayItem` (`self.Discs`) (`self.SelectedDiscIndex`))))

(fn `SetSelectedDiscHighlight`
  (params (bEnabled :type Boolean))
  (`self.SetHighlight` bEnabled (`self.GetSelectedDisc`)))

(fn `UserConstructionScript`)