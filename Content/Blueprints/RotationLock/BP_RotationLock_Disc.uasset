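; A rotating disc for a rotation lock, stepping between numbered faces and reporting the symbol currently selected.
; Rotate moves the face index up or down with wraparound and derives a target roll from the face count.
; Tick smoothly lerps the relative rotation toward that roll along the shortest path.
; GetCurrentSymbol maps the selected index to one of five enum symbols.
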(event `self.ReceiveTick`
  (params (DeltaSeconds :type "Float (single-precision)"))
  (`self.K2_SetRelativeRotation` (`KismetMathLibrary.RLerp` (`self.RelativeRotation`) (`KismetMathLibrary.MakeRotator` (`self.TargetRot`)) (* (`GameplayStatics.GetWorldDeltaSeconds`) 10.0) true)))

(event `Rotate`
  (params (bUp :type Boolean))
  (bind _output_get (set `self.CurrentSelectedFace` (`self.ClampSelectedFace` (+ (`self.CurrentSelectedFace`) (`KismetMathLibrary.SelectInt` 1 -1 bUp)))))
  (set `self.TargetRot` (* (`KismetMathLibrary.Conv_IntToDouble` _output_get) (/ 360.0 (`KismetMathLibrary.Conv_IntToDouble` (`self.NumFaces`))) -1.0)))

(fn `ClampSelectedFace`
  (params (index :type Integer))
  (returns (ReturnValue :type Integer))
  (locals (ClampedIndex :type Integer))
  (set `local.ClampedIndex` index)
  (`|ExecutionSequence`
    (:`then_0`
      (if (> (`local.ClampedIndex`) (- (`self.NumFaces`) 1))
        (set `local.ClampedIndex` 0)))
    (:`then_1`
      (if (< (`local.ClampedIndex`) 0)
        (set `local.ClampedIndex` (- (`self.NumFaces`) 1))))
    (:`then_2`
      (return (`local.ClampedIndex`)))))

(fn `GetCurrentSymbol`
  (returns (Symbol :type "/Game/Blueprints/RotationLock/ERotationLockSymbol Enum"))
  (return (select `int` (`self.CurrentSelectedFace`) :`0` "NewEnumerator0" :`1` "NewEnumerator1" :`2` "NewEnumerator2" :`3` "NewEnumerator3" :`4` "NewEnumerator4" :!type "/Game/Blueprints/RotationLock/ERotationLockSymbol Enum")))