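; Keypad puzzle pawn that the player interacts with to enter a code on a twelve-button pad.
; Navigation input moves a wrapping index through the button array in steps of one or three, highlighting the selection with an overlay material.
; Digits append to the display up to the code's length, while Cancel clears it.
; Confirm clears a wrong code or returns to the character on a correct one; the unlock action is still a TODO.
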(event `self.ReceiveBeginPlay`
  ;[1 1 1] Setup
  (`parent.ReceiveBeginPlay`)
  (set `self.Buttons` (`|MakeArray` (`self.Button_1`) (`self.Button_2`) (`self.Button_3`) (`self.Button_4`) (`self.Button_5`) (`self.Button_6`) (`self.Button_7`) (`self.Button_8`) (`self.Button_9`) (`self.Button_Cancel`) (`self.Button_0`) (`self.Button_Confirm`)))
  (`self.ClearDisplay`))

(event `/Game/Blueprints/InteractionInterface.Interact`
  (params (PlayerCharacter :type "/Game/Blueprints/BP_FirstPersonCharacter Object Reference"))
  ;[1 1 1] Possess & UnPossess
  (`parent.Interact` PlayerCharacter)
  (`self.UpdateHighlightOfSelectedButton` true))

(event `EnhancedInput|/Game/Input/Actions/IA_ExitPuzzle`
  (params (ActionValue :type Boolean) (ElapsedSeconds :type "Float (double-precision)") (TriggeredSeconds :type "Float (double-precision)") (InputAction :type "InputAction Object Reference" :default "/Game/Input/Actions/IA_ExitPuzzle.IA_ExitPuzzle"))
  ;[1 1 1] Possess & UnPossess
  (:`Triggered`
    (`self.Return to Character`)))

(event `self.Return to Character`
  ;[1 1 1] Possess & UnPossess
  (`parent.Return to Character`)
  (`self.UpdateHighlightOfSelectedButton` false))

(event `EnhancedInput|/Game/Input/Actions/IA_NavigateRight`
  (params (ActionValue :type Boolean) (ElapsedSeconds :type "Float (double-precision)") (TriggeredSeconds :type "Float (double-precision)") (InputAction :type "InputAction Object Reference" :default "/Game/Input/Actions/IA_NavigateRight.IA_NavigateRight"))
  (:`Triggered`
    (`self.Navigate Buttons` 1)))

(event `EnhancedInput|/Game/Input/Actions/IA_NavigateLeft`
  (params (ActionValue :type Boolean) (ElapsedSeconds :type "Float (double-precision)") (TriggeredSeconds :type "Float (double-precision)") (InputAction :type "InputAction Object Reference" :default "/Game/Input/Actions/IA_NavigateLeft.IA_NavigateLeft"))
  (:`Triggered`
    (`self.Navigate Buttons` -1)))

(event `EnhancedInput|/Game/Input/Actions/IA_NavigateDown`
  (params (ActionValue :type Boolean) (ElapsedSeconds :type "Float (double-precision)") (TriggeredSeconds :type "Float (double-precision)") (InputAction :type "InputAction Object Reference" :default "/Game/Input/Actions/IA_NavigateDown.IA_NavigateDown"))
  (:`Triggered`
    (`self.Navigate Buttons` 3)))

(event `EnhancedInput|/Game/Input/Actions/IA_NavigateUp`
  (params (ActionValue :type Boolean) (ElapsedSeconds :type "Float (double-precision)") (TriggeredSeconds :type "Float (double-precision)") (InputAction :type "InputAction Object Reference" :default "/Game/Input/Actions/IA_NavigateUp.IA_NavigateUp"))
  (:`Triggered`
    (`self.Navigate Buttons` -3)))

(event `EnhancedInput|/Game/Input/Actions/IA_Interact`
  (params (ActionValue :type Boolean) (ElapsedSeconds :type "Float (double-precision)") (TriggeredSeconds :type "Float (double-precision)") (InputAction :type "InputAction Object Reference" :default "/Game/Input/Actions/IA_Interact.IA_Interact"))
  (:`Triggered`
    (if (== (`self.GetSelectedButton`) (`self.Button_Confirm`))
      ;[1 1 1] Check if code correct
      (if (`self.IsCodeCorrect`)
        ;;[1 1 1] TODO: Open door / unlock secret / ....
        (`self.Return to Character`)
        (else
          (`self.ClearDisplay`)))
      (elif (== (`self.GetSelectedButton`) (`self.Button_Cancel`))
        ;[1 1 1] Cancel button -> Clear display
        (`self.ClearDisplay`)
        (else
          ;[1 1 1] Add number to display
          (if (not (`self.IsCodeComplete`))
            (`self.AddToDisplay` (`/Game/Blueprints/Keypad/BP_KeypadButton.ButtonLabel` (`self.GetSelectedButton`)))))))))

(fn `AddToDisplay`
  (params (NumberToAdd :type String))
  (bind _codedisplay (`self.CodeDisplay`))
  (`TextRenderComponent.K2_SetText` _codedisplay (`KismetTextLibrary.Conv_StringToText` (`KismetStringLibrary.Concat_StrStr` (`KismetTextLibrary.Conv_TextToString` (`TextRenderComponent.Text` _codedisplay)) NumberToAdd))))

(fn `ClearDisplay`
  (`TextRenderComponent.K2_SetText` (`self.CodeDisplay`) (`KismetTextLibrary.Conv_StringToText` "")))

(fn `GetSelectedButton`
  (returns (Output :type "/Game/Blueprints/Keypad/BP_KeypadButton Object Reference"))
  (return (`|GetArrayItem` (`self.Buttons`) (`self.CurrentButtonIndex`))))

(fn `IsCodeComplete`
  (returns (ReturnValue :type Boolean))
  (return (== (`KismetStringLibrary.Len` (`KismetTextLibrary.Conv_TextToString` (`TextRenderComponent.Text` (`self.CodeDisplay`)))) (`KismetStringLibrary.Len` (`self.CorrectCode`)))))

(fn `IsCodeCorrect`
  (returns (ReturnValue :type Boolean))
  (return (`KismetStringLibrary.EqualEqual_StrStr` (`KismetTextLibrary.Conv_TextToString` (`TextRenderComponent.Text` (`self.CodeDisplay`))) (`self.CorrectCode`))))

(fn `Navigate Buttons`
  (params (Direction :type Integer))
  (`self.UpdateHighlightOfSelectedButton` false)
  (set `self.CurrentButtonIndex` (+ (`self.CurrentButtonIndex`) Direction))
  (`|ExecutionSequence`
    (:`then_0`
      ;[1 1 1] Make sure index is not too high
      (if (> (`self.CurrentButtonIndex`) (`KismetArrayLibrary.Array_LastIndex` (`self.Buttons`)))
        (set `self.CurrentButtonIndex` (- (`self.CurrentButtonIndex`) (`KismetArrayLibrary.Array_Length` (`self.Buttons`))))))
    (:`then_1`
      ;[1 1 1] Make sure index is not too low
      (if (< (`self.CurrentButtonIndex`) 0)
        (set `self.CurrentButtonIndex` (+ (`self.CurrentButtonIndex`) (`KismetArrayLibrary.Array_Length` (`self.Buttons`))))))
    (:`then_2`
      ;[1 1 1] Enable highlicht
      (`self.UpdateHighlightOfSelectedButton` true))))

(fn `UpdateHighlightOfSelectedButton`
  (params (bEnable :type Boolean))
  (`MeshComponent.SetOverlayMaterial` (`self.GetSelectedButton`) (select `bool` bEnable :`true` "/Game/Materials/MI_ButtonHighlight.MI_ButtonHighlight" :!type "MaterialInterface Object Reference")))

(fn `UserConstructionScript`)