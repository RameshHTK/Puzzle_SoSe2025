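; BP_KeypadButton is a mesh component for a single keypad button that displays its own number and can be highlighted.
; On BeginPlay it adds a text render component to its owner, attaches it to itself with an offset along X, and sets its text from the Number variable.
; SetHighlight toggles a highlight overlay material on the button, clearing it when disabled.
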(event `self.ReceiveBeginPlay`
  (bind _returnvalue (`|AddComponentByClass` :`self` (`self.GetOwner`) :`Class` "/Script/Engine.TextRenderComponent"))
  (`self.K2_AttachToComponent` _returnvalue self "None" "KeepRelative" "KeepRelative" "KeepRelative" true)
  (`self.K2_SetRelativeLocation` _returnvalue (80.0 0.0 0.0) false false)
  (`TextRenderComponent.SetTextRenderColor` _returnvalue (make `Color` 0))
  (`TextRenderComponent.K2_SetText` _returnvalue (`KismetTextLibrary.Conv_StringToText` (`self.Number`))))

(event `SetHighlight`
  (params (bEnabled :type Boolean))
  (`self.SetOverlayMaterial` (select `bool` bEnabled :`true` "/Game/Materials/MI_ButtonHighlight.MI_ButtonHighlight" :!type "MaterialInterface Object Reference")))